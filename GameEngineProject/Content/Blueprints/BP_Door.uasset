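; BP_Door is a door actor that slides its Door component between a closed and an open world location.
; The OpenDoor and CloseDoor events each play their own timeline, MovingDoor and ClosingDoor, whose Alpha drives a lerp between the two stored positions.
; Each timeline plays forward with swapped endpoints instead of reversing, and the movement is applied without sweep.
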(event `OpenDoor`
  (bind (_direction _alpha) (`Timeline|MovingDoor`)
    (:`Update`
      (`SceneComponent.K2_SetWorldLocation` (`self.Door`) (`KismetMathLibrary.VLerp` (`self.ClosedDoorLocation`) (`self.OpenDoorLocation`) _alpha) false false))))

(event `CloseDoor`
  (bind (_direction _alpha) (`Timeline|ClosingDoor`)
    (:`Update`
      (`SceneComponent.K2_SetWorldLocation` (`self.Door`) (`KismetMathLibrary.VLerp` (`self.OpenDoorLocation`) (`self.ClosedDoorLocation`) _alpha) false false))))

(fn `UserConstructionScript`)