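; Deadly trunk hazard that calls Death on the FirstPersonCharacter whenever it overlaps the actor.
; ActivateTrunk lifts the mesh and trigger area together by timeline lerp, then starts a looping spin timer and a vertical movement timeline with adjustable play rate.
; Other events raise the trunk, shift it along X to punish the player, or lower it to disable it.
; The spin timer is never cleared, and the kill ignores IsActive.
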(event `SpeedUp`
  (params (NewSpeed :type "Float (double-precision)"))
  ;[1 1 1] Speed Up
  (`TimelineComponent.SetPlayRate` (`self.MoveTimeLine`) NewSpeed))

(event `ActivateTrunk`
  (bind (_returnvalue_x _returnvalue_y) (`KismetMathLibrary.BreakVector` (`self.K2_GetActorLocation`)))
  (bind (_returnvalue_x_2 _returnvalue_y_2) (`KismetMathLibrary.BreakVector` (`self.K2_GetActorLocation`)))
  ;[1 1 1] Activate Trunk
  ;;[1 1 1] Spawn
  (bind (_direction _spawntrack) (`Timeline|Timeline_0`)
    (:`Update`
      (`SceneComponent.K2_SetWorldLocation` (`self.DeadlyTrunkMesh`) (`KismetMathLibrary.VLerp` (`self.K2_GetActorLocation`) (`KismetMathLibrary.MakeVector` _returnvalue_x_2 _returnvalue_y_2 330.0) _spawntrack) false false)
      (`SceneComponent.K2_SetWorldLocation` (`self.TriggerArea`) (`KismetMathLibrary.VLerp` (`self.K2_GetActorLocation`) (`KismetMathLibrary.MakeVector` _returnvalue_x_2 _returnvalue_y_2 330.0) _spawntrack) false false))
    (:`Finished`
      (set `self.IsActive` true)
      ;;[1 1 1] Rotate Trunk
      (`KismetSystemLibrary.K2_SetTimerDelegate` (delegate `Rotate Trunk`) 0.0025 true)
      ;;[1 1 1] Move Trunk up and down
      (bind (_direction_2 _first_move) (`Timeline|MoveTimeLine`)
        (:`Update`
          (if (`self.IsActive`)
            (`SceneComponent.K2_SetWorldLocation` (`self.DeadlyTrunkMesh`) (`KismetMathLibrary.VLerp` (`self.K2_GetActorLocation`) (`KismetMathLibrary.MakeVector` _returnvalue_x _returnvalue_y 330.0) _first_move) false false)
            (`SceneComponent.K2_SetWorldLocation` (`self.TriggerArea`) (`KismetMathLibrary.VLerp` (`self.K2_GetActorLocation`) (`KismetMathLibrary.MakeVector` _returnvalue_x _returnvalue_y 330.0) _first_move) false false)))))))

(event `DisableTrunk`
  (bind (_returnvalue_x _returnvalue_y) (`KismetMathLibrary.BreakVector` (`self.K2_GetActorLocation`)))
  ;[1 1 1] Disable Trunk
  (`TimelineComponent.Stop` (`self.MoveTimeLine`))
  (bind (_direction _spawntrack) (`Timeline|Timeline_3`)
    (:`Update`
      (`SceneComponent.K2_SetWorldLocation` (`self.DeadlyTrunkMesh`) (`KismetMathLibrary.VLerp` (`self.K2_GetActorLocation`) (`KismetMathLibrary.MakeVector` _returnvalue_x _returnvalue_y -480.0) _spawntrack) false false)
      (`SceneComponent.K2_SetWorldLocation` (`self.TriggerArea`) (`KismetMathLibrary.VLerp` (`self.K2_GetActorLocation`) (`KismetMathLibrary.MakeVector` _returnvalue_x _returnvalue_y -480.0) _spawntrack) false false))
    (:`Finished`
      (set `self.IsActive` false))))

(event `Rotate Trunk`
  ;[1 1 1] Activate Trunk
  ;;[1 1 1] Rotate Trunk
  (`SceneComponent.K2_AddWorldRotation` (`self.DeadlyTrunkMesh`) (struct :`Yaw` 1.0) false false))

(event `MoveToLocation`
  (params (location :type "Float (double-precision)"))
  (bind _deadlytrunkmesh (`self.DeadlyTrunkMesh`))
  (bind (_returnvalue_x _returnvalue_y _returnvalue_z) (`KismetMathLibrary.BreakVector` (`SceneComponent.K2_GetComponentLocation` _deadlytrunkmesh)))
  ;[1 1 1] Punish player
  (bind (_direction _spawntrack) (`Timeline|Timeline_2`)
    (:`Update`
      (`SceneComponent.K2_SetWorldLocation` (`self.DeadlyTrunkMesh`) (`KismetMathLibrary.VLerp` (`SceneComponent.K2_GetComponentLocation` _deadlytrunkmesh) (`KismetMathLibrary.MakeVector` location _returnvalue_y _returnvalue_z) _spawntrack) false false)
      (`SceneComponent.K2_SetWorldLocation` (`self.TriggerArea`) (`KismetMathLibrary.VLerp` (`SceneComponent.K2_GetComponentLocation` _deadlytrunkmesh) (`KismetMathLibrary.MakeVector` location _returnvalue_y _returnvalue_z) _spawntrack) false false))))

(event `RaiseTrunk`
  (bind _deadlytrunkmesh (`self.DeadlyTrunkMesh`))
  (bind (_returnvalue_x _returnvalue_y) (`KismetMathLibrary.BreakVector` (`SceneComponent.K2_GetComponentLocation` _deadlytrunkmesh)))
  ;[1 1 1] Raise Trunk
  (set `self.IsActive` false)
  (bind (_direction _spawntrack) (`Timeline|Timeline_1`)
    (:`Update`
      (`SceneComponent.K2_SetWorldLocation` (`self.DeadlyTrunkMesh`) (`KismetMathLibrary.VLerp` (`SceneComponent.K2_GetComponentLocation` _deadlytrunkmesh) (`KismetMathLibrary.MakeVector` _returnvalue_x _returnvalue_y 320.0) _spawntrack) false false)
      (`SceneComponent.K2_SetWorldLocation` (`self.TriggerArea`) (`KismetMathLibrary.VLerp` (`SceneComponent.K2_GetComponentLocation` _deadlytrunkmesh) (`KismetMathLibrary.MakeVector` _returnvalue_x _returnvalue_y 320.0) _spawntrack) false false))))

(event `self.ReceiveActorBeginOverlap`
  (params (OtherActor :type "Actor Object Reference"))
  ;[1 1 1] Death
  (bind _asfirst_person_character (cast `/Game/FirstPersonBP/Blueprints/FirstPersonCharacter` OtherActor))
  (`/Game/FirstPersonBP/Blueprints/FirstPersonCharacter.Death` _asfirst_person_character))

(fn `UserConstructionScript`)