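; BP_Wall_Trap is a trap actor with left and right walls that slide toward opposite Y directions to close on command.
; BeginPlay caches each wall's world start location and an end point offset along world Y.
; The CloseWall custom event plays a timeline whose alpha lerps both walls between those points without sweeping, and nothing in the file reverses it.
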(event `self.ReceiveBeginPlay`
  (bind _returnvalue (`SceneComponent.K2_GetComponentLocation` (`self.WallTrapLeft`)))
  (bind _returnvalue_2 (`SceneComponent.K2_GetComponentLocation` (`self.WallTrapRight`)))
  (set `self.LeftWallStartLocation` _returnvalue)
  (set `self.LeftWallFinalLocation` (+ _returnvalue (0.0 400.0 0.0)))
  (set `self.RightWallStartLocation` _returnvalue_2)
  (set `self.RightWallFinalLocation` (+ _returnvalue_2 (0.0 -400.0 0.0))))

(event `CloseWall`
  (bind (_direction _alpha) (`Timeline|Timeline_0`)
    (:`Update`
      (`SceneComponent.K2_SetWorldLocation` (`self.WallTrapLeft`) (`KismetMathLibrary.VLerp` (`self.LeftWallStartLocation`) (`self.LeftWallFinalLocation`) _alpha) false false)
      (`SceneComponent.K2_SetWorldLocation` (`self.WallTrapRight`) (`KismetMathLibrary.VLerp` (`self.RightWallStartLocation`) (`self.RightWallFinalLocation`) _alpha) false false))))

(fn `UserConstructionScript`)