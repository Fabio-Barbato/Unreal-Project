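; BP_Door2 is a double-door actor that swings both leaves open when its OpenDoor event is called.
; OpenDoor plays the OpeningDoor timeline, whose Alpha output lerps LeftDoor and RightDoor between their stored closed and open rotations, set in world space.
; The file has no closing logic or trigger of its own, as BeginPlay, overlap and Tick are unused.
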(event `OpenDoor`
  (bind (_direction _alpha) (`Timeline|OpeningDoor`)
    (:`Update`
      (`SceneComponent.K2_SetWorldRotation` (`self.LeftDoor`) (`KismetMathLibrary.RLerp` (`self.LeftDoorClosedRotation`) (`self.LeftDoorOpenRotation`) _alpha) false false)
      (`SceneComponent.K2_SetWorldRotation` (`self.RightDoor`) (`KismetMathLibrary.RLerp` (`self.RightDoorClosedRotation`) (`self.RightDoorOpenRotation`) _alpha) false false))))

(fn `UserConstructionScript`)