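; Interactable torch actor with fire, light and text render components that disappears when the player uses it.
; UserInteract runs once through a DoOnce, fires the TorchInteract dispatcher, then hides the torch, fire and light via visibility and the text via hidden-in-game.
; A separate TorchOn function lights the torch by clearing hidden-in-game on the fire and light.
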(event `/Game/Blueprints/InteractInterface.UserInteract`
  (`/Engine/EditorBlueprintResources/StandardMacros.DoOnce` false
    (:`Completed`
      (`self.TorchInteract`)
      (`SceneComponent.SetVisibility` (`self.Torch`) false false)
      (`SceneComponent.SetVisibility` (`self.Fire`) false false)
      (`SceneComponent.SetVisibility` (`self.FireLight`) false false)
      (`SceneComponent.SetHiddenInGame` (`self.TextRender`) true false))))

(fn `Torch On`
  (`SceneComponent.SetHiddenInGame` (`self.Fire`) false false)
  (`SceneComponent.SetHiddenInGame` (`self.FireLight`) false false))

(fn `UserConstructionScript`)