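; Interactable gold chest that holds a paper message and ends the game once that message is dismissed.
; The first interaction swings the lid open with a timeline; later ones flip-flop between showing PaperWidget and removing all widgets, toggling the character's IsPaperTaken with a sound.
; Closing the paper calls EndGame on the character.
; BeginPlay writes the message to a text render, and construction creates a dynamic material for body and lid.
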(event `/Game/Blueprints/InterfaceAndAbstarct/InteractInterface.UserInteract`
  (bind _dyntimelinecol (`self.DynTimelineCol`))
  (if (`self.ChestOpened`)
    ;[1 1 1] Every time the player interact with the message, it appears PaperWidget on the screen. If the player interact again, the widget disappers.
    ; The constructor set the widget's message. When the player interacts, it plays a sound.
    (bind _asfirst_person_character (cast `/Game/FirstPersonBP/Blueprints/FirstPersonCharacter` (`GameplayStatics.GetPlayerCharacter` 0)))
    (`/Engine/EditorBlueprintResources/StandardMacros.FlipFlop`
      (:`A`
        (bind _returnvalue (`|GenericCreateObject` "/Game/Blueprints/InterfaceAndAbstarct/PaperWidget.PaperWidget_C" _asfirst_person_character))
        (set `/Game/Blueprints/InterfaceAndAbstarct/PaperWidget.MessageWidget` (`self.Message`) _returnvalue)
        (`UserWidget.AddToViewport` _returnvalue 0)
        (set `/Game/FirstPersonBP/Blueprints/FirstPersonCharacter.IsPaperTaken` true _asfirst_person_character)
        (`GameplayStatics.PlaySound2D` "/Game/Sounds/SC_PaperTaken.SC_PaperTaken" 1.0 1.0 0.0 null null)
        (`TimelineComponent.ReverseFromEnd` _dyntimelinecol)
        (`TimelineComponent.Stop` _dyntimelinecol))
      (:`B`
        (`WidgetLayoutLibrary.RemoveAllWidgets`)
        (set `/Game/FirstPersonBP/Blueprints/FirstPersonCharacter.IsPaperTaken` false _asfirst_person_character)
        (`GameplayStatics.PlaySound2D` "/Game/Sounds/SC_PaperTaken.SC_PaperTaken" 1.0 2.0 0.0 null null)
        (`/Game/FirstPersonBP/Blueprints/FirstPersonCharacter.EndGame` _asfirst_person_character)))
    (else
      (bind (_direction _opentack) (`Timeline|OpenChest`)
        (:`Update`
          (`SceneComponent.K2_SetRelativeRotation` (`self.ChestHead`) (`KismetMathLibrary.RLerp` (struct) (struct :`Roll` -90.0) _opentack) false false))
        (:`Finished`
          (set `self.ChestOpened` true))))))

(event `self.ReceiveBeginPlay`
  ;[1 1 1] Set message on BeginPlay
  (`TextRenderComponent.K2_SetText` (`self.MessageTextRender`) (`KismetTextLibrary.Conv_StringToText` (`self.Message`))))

(fn `UserConstructionScript`
  (bind _returnvalue (`PrimitiveComponent.CreateDynamicMaterialInstance` (`self.ChestBody`) 0 null "None"))
  (bind _output_get (set `self.DynamicCol` _returnvalue))
  (`PrimitiveComponent.CreateDynamicMaterialInstance` (`self.ChestHead`) 0 _output_get "None"))