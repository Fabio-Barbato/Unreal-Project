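; Neon floor tile that starts randomly safe or unsafe, then flips state and emissive color on a fixed delay loop via a dynamic material.
; Unsafe tiles drop the first-person character immediately by switching collision to overlap.
; Safe tiles chain timers through two escalating camera shakes with sound before dropping the player, cancelled on end overlap.
; Example tiles keep their set state, and unsafe ones sink via timeline after non-player overlaps.
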(event `self.ReceiveBeginPlay`
  (bind _tilematerial (`self.TileMaterial`))
  ;[1 1 1] Cambio stato e colore della piastrella
  (if (not (`self.IsExample`))
    (if (== (`KismetMathLibrary.RandomIntegerInRange` 1 2) 1)
      (set `self.TileState` "NewEnumerator0")
      (else
        (set `self.TileState` "NewEnumerator1")))
    (`KismetSystemLibrary.Delay` 4.1 :!label _label)
    (switch `/Game/Blueprints/Enum_TileState` (`self.TileState`)
      (:`NewEnumerator0`
        (set `self.TileState` "NewEnumerator1")
        (`MaterialInstanceDynamic.SetVectorParameterValue` _tilematerial "Emissive color 01" (struct :`R` 0.35 :`G` 0.041 :`A` 1.0))
        (goto _label))
      (:`NewEnumerator1`
        (set `self.TileState` "NewEnumerator0")
        (`MaterialInstanceDynamic.SetVectorParameterValue` _tilematerial "Emissive color 01" (struct :`R` 0.56 :`G` 2.96 :`B` 4.0 :`A` 1.0))
        (goto _label)))))

(event `self.ReceiveActorBeginOverlap`
  (params (OtherActor :type "Actor Object Reference"))
  (bind _tilestate (`self.TileState`))
  (bind _tile (`self.Tile`))
  ;[1 1 1] BeginOverlap
  (cast `/Game/FirstPersonBP/Blueprints/FirstPersonCharacter` OtherActor
    (:`then`
      (switch `/Game/Blueprints/Enum_TileState` _tilestate
        (:`NewEnumerator0`
          (bind _returnvalue (`KismetSystemLibrary.K2_SetTimerDelegate` (delegate `FirstShake`) 4.0))
          (set `self.FirstShakeTimerHandler` _returnvalue))
        (:`NewEnumerator1`
          (`PrimitiveComponent.SetCollisionResponseToAllChannels` _tile "ECR_Overlap"))))
    (:`CastFailed`
      (if (and (`|EnumEquality` _tilestate "NewEnumerator1") (`self.IsExample`))
        (`KismetSystemLibrary.Delay` 5.3)
        (bind (_direction _newtrack_0) (`Timeline|Timeline_0`)
          (:`Update`
            (`SceneComponent.K2_SetRelativeLocation` _tile (`KismetMathLibrary.MakeVector` 0.0 0.0 (`KismetMathLibrary.Lerp` 0.0 -700.0 _newtrack_0)) false false)))))))

(event `FirstShake`
  ;[1 1 1] BeginOverlap
  (bind _returnvalue (`GameplayStatics.SpawnSound2D` "/Game/Sounds/SC_FirstShake.SC_FirstShake" 1.0 1.0 0.0 null))
  (set `self.SoundShake` _returnvalue)
  (`PlayerController.ClientStartCameraShake` :`self` (`GameplayStatics.GetPlayerController` 0) :`Shake` "/Game/Blueprints/BP_FirstShake.BP_FirstShake_C")
  (bind _returnvalue_2 (`KismetSystemLibrary.K2_SetTimerDelegate` (delegate `SecondShake`) 4.0))
  (set `self.SecondShakeTimerHandler` _returnvalue_2))

(event `SecondShake`
  (bind _returnvalue (`GameplayStatics.GetPlayerController` 0))
  ;[1 1 1] BeginOverlap
  (bind _returnvalue_2 (`GameplayStatics.SpawnSound2D` "/Game/Sounds/SC_FirstShake.SC_FirstShake" 1.25 2.0 0.0 null))
  (set `self.SoundShake` _returnvalue_2)
  (`PlayerController.ClientStopCameraShake` _returnvalue "/Game/Blueprints/BP_FirstShake.BP_FirstShake_C" true)
  (`PlayerController.ClientStartCameraShake` :`self` _returnvalue :`Shake` "/Game/Blueprints/BP_SecondShake.BP_SecondShake_C")
  (bind _returnvalue_3 (`KismetSystemLibrary.K2_SetTimerDelegate` (delegate `GameOver`) 4.0))
  (set `self.GameOverTimerHandler` _returnvalue_3))

(event `GameOver`
  ;[1 1 1] BeginOverlap
  (`PlayerController.ClientStopCameraShake` (`GameplayStatics.GetPlayerController` 0) "/Game/Blueprints/BP_SecondShake.BP_SecondShake_C" true)
  (`PrimitiveComponent.SetCollisionResponseToAllChannels` (`self.Tile`) "ECR_Overlap"))

(event `self.ReceiveActorEndOverlap`
  (params (OtherActor :type "Actor Object Reference"))
  (bind _soundshake (`self.SoundShake`))
  ;[1 1 1] EndOverlap
  (`KismetSystemLibrary.K2_ClearAndInvalidateTimerHandle` (`self.FirstShakeTimerHandler`))
  (`KismetSystemLibrary.K2_ClearAndInvalidateTimerHandle` (`self.SecondShakeTimerHandler`))
  (`KismetSystemLibrary.K2_ClearAndInvalidateTimerHandle` (`self.GameOverTimerHandler`))
  (`PlayerController.ClientStopCameraShake` (`GameplayStatics.GetPlayerController` 0) "/Script/Engine.MatineeCameraShake" true)
  (if (`KismetSystemLibrary.IsValid` _soundshake)
    (`AudioComponent.Stop` _soundshake)))

(fn `UserConstructionScript`
  (bind _tilematerial (`self.TileMaterial`))
  (bind _returnvalue (`PrimitiveComponent.CreateDynamicMaterialInstance` (`self.Tile`) 0 "/Game/Material/M_Tech_Hex_Inst.M_Tech_Hex_Inst" "None"))
  (set `self.TileMaterial` _returnvalue)
  (if (`self.IsExample`)
    (if (`|EnumEquality` (`self.TileState`) "NewEnumerator0")
      (`MaterialInstanceDynamic.SetVectorParameterValue` _tilematerial "Emissive color 01" (struct :`R` 0.56 :`G` 2.96 :`B` 4.0 :`A` 1.0))
      (else
        (`MaterialInstanceDynamic.SetVectorParameterValue` _tilematerial "Emissive color 01" (struct :`R` 0.35 :`G` 0.041 :`A` 1.0))))))