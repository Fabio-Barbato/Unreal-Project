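; BP_Cart is an interactable cart that slides to a fixed world X position when the player uses it.
; Interaction plays a sound, stops the color timeline, marks it interacted, and runs a timeline lerping the cart mesh from the actor's location.
; A looping timer spins the four wheel meshes, with no logic to stop it.
; Construction creates a dynamic material on the cart and uses it as each wheel's source material.
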(event `/Game/Blueprints/InterfaceAndAbstarct/InteractInterface.UserInteract`
  (bind (_returnvalue_x _returnvalue_y _returnvalue_z) (`KismetMathLibrary.BreakVector` (`self.K2_GetActorLocation`)))
  (bind _dyntimelinecol (`self.DynTimelineCol`))
  (`GameplayStatics.PlaySound2D` "/Game/Sounds/CartMove.CartMove" 1.0 1.0 0.0 null null)
  (`TimelineComponent.ReverseFromEnd` _dyntimelinecol)
  (`TimelineComponent.Stop` _dyntimelinecol)
  (set `self.IsInteracted` true)
  (bind _returnvalue (`KismetSystemLibrary.K2_SetTimer` null "RotationWheel" 0.01 true))
  (bind (_direction _newtrack_0) (`Timeline|MoveCart`)
    (:`Update`
      (`SceneComponent.K2_SetWorldLocation` (`self.CartMesh`) (`KismetMathLibrary.VLerp` (`self.K2_GetActorLocation`) (`KismetMathLibrary.MakeVector` 4850.0 _returnvalue_y _returnvalue_z) _newtrack_0) false false))))

(fn `RotationWheel`
  (`SceneComponent.K2_AddWorldRotation` (`self.WheelMeshAL`) (struct :`Pitch` -1.0) false false)
  (`SceneComponent.K2_AddWorldRotation` (`self.WheelMeshBL`) (struct :`Pitch` -1.0) false false)
  (`SceneComponent.K2_AddWorldRotation` (`self.WheelMeshBR`) (struct :`Pitch` -1.0) false false)
  (`SceneComponent.K2_AddWorldRotation` (`self.WheelMeshAR`) (struct :`Pitch` -1.0) false false))

(fn `UserConstructionScript`
  (bind _returnvalue (`PrimitiveComponent.CreateDynamicMaterialInstance` (`self.CartMesh`) 0 null "None"))
  (bind _output_get (set `self.DynamicCol` _returnvalue))
  (`PrimitiveComponent.CreateDynamicMaterialInstance` (`self.WheelMeshAL`) 0 _output_get "None")
  (`PrimitiveComponent.CreateDynamicMaterialInstance` (`self.WheelMeshBL`) 0 _output_get "None")
  (`PrimitiveComponent.CreateDynamicMaterialInstance` (`self.WheelMeshBR`) 0 _output_get "None")
  (`PrimitiveComponent.CreateDynamicMaterialInstance` (`self.WheelMeshAR`) 0 _output_get "None"))