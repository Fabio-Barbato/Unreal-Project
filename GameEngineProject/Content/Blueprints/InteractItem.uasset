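; InteractItem is an interactable item Blueprint that shows a text label when the FirstPersonCharacter overlaps it and hides it when the overlap ends.
; On overlap begin, the TextRender becomes visible and starts turning toward the player camera through the LookPlayer function, which uses FindLookAtRotation.
; A short non-looping timer re-arms itself while the text stays visible, updating the billboard rotation without Event Tick.
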(event `self.ReceiveBeginPlay`)

(event `Event LookPlayer`
  (bind _textrender (`self.TextRender`))
  (`self.LookPlayer` _textrender :!label _label)
  (if (`SceneComponent.IsVisible` _textrender)
    (`KismetSystemLibrary.K2_SetTimerDelegate` (delegate `Event LookPlayer`) 0.05)))

(event `self.ReceiveActorBeginOverlap`
  (params (OtherActor :type "Actor Object Reference"))
  (cast `/Game/FirstPersonBP/Blueprints/FirstPersonCharacter` OtherActor)
  (`SceneComponent.SetVisibility` (`self.TextRender`) true false)
  (goto _label))

(event `self.ReceiveActorEndOverlap`
  (params (OtherActor :type "Actor Object Reference"))
  (cast `/Game/FirstPersonBP/Blueprints/FirstPersonCharacter` OtherActor)
  (`SceneComponent.SetVisibility` (`self.TextRender`) false false))

(fn `LookPlayer`
  (params (SceneComponent :type "SceneComponent Object Reference"))
  (`SceneComponent.K2_SetWorldRotation` SceneComponent (`KismetMathLibrary.FindLookAtRotation` (`SceneComponent.K2_GetComponentLocation` SceneComponent) (`PlayerCameraManager.GetCameraLocation` (`GameplayStatics.GetPlayerCameraManager` 0))) false false))

(fn `UserConstructionScript`)