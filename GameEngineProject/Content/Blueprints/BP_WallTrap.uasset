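; BP_WallTrap is a trap actor with left and right walls that slide in opposite directions when triggered.
; The ActivateTrap event, with no caller in this graph, records each wall's start and a target offset along world Y, so actor rotation is ignored.
; A timeline then lerps both walls to their targets without sweep, and the graph has no reset.
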(event `ActivateTrap`
  (bind (_returnvalue_x _returnvalue_y _returnvalue_z) (`KismetMathLibrary.BreakVector` (`SceneComponent.K2_GetComponentLocation` (`self.WallTrapLeft`))))
  (bind (_returnvalue_x_2 _returnvalue_y_2 _returnvalue_z_2) (`KismetMathLibrary.BreakVector` (`SceneComponent.K2_GetComponentLocation` (`self.WallTrapRight`))))
  (set `self.LeftWallStartLocation` (`KismetMathLibrary.MakeVector` _returnvalue_x _returnvalue_y _returnvalue_z))
  (set `self.LeftWallFinalLocation` (`KismetMathLibrary.MakeVector` _returnvalue_x (+ _returnvalue_y 500.0) _returnvalue_z))
  (set `self.RightWallStartLocation` (`KismetMathLibrary.MakeVector` _returnvalue_x_2 _returnvalue_y_2 _returnvalue_z_2))
  (set `self.RightWallFinalLocation` (`KismetMathLibrary.MakeVector` _returnvalue_x_2 (- _returnvalue_y_2 500.0) _returnvalue_z_2))
  (bind (_direction _alpha) (`Timeline|Timeline_0`)
    (:`Update`
      (`SceneComponent.K2_SetWorldLocation` (`self.WallTrapLeft`) (`KismetMathLibrary.VLerp` (`self.LeftWallStartLocation`) (`self.LeftWallFinalLocation`) _alpha) false false)
      (`SceneComponent.K2_SetWorldLocation` (`self.WallTrapRight`) (`KismetMathLibrary.VLerp` (`self.RightWallStartLocation`) (`self.RightWallFinalLocation`) _alpha) false false))))

(fn `UserConstructionScript`)