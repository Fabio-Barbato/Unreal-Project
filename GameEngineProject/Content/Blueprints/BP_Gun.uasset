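; Dart gun trap that fires on a looping timer and kills the first-person character.
; Before each shot, a timeline drives the red channel of a dynamic emissive material on the gun mesh as a warning.
; When it finishes, a shot sound plays and a second timeline slides the dart mesh along local Y.
; Character overlaps with the dart trigger area call Death; other character overlaps play a flying-arrow sound.
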(event `Fire`
  ;[1 1 1] Change color before shot
  (bind _returnvalue (`PrimitiveComponent.CreateDynamicMaterialInstance` (`self.GunMesh`) 0 "/Game/Material/M_Metal_Rust_EmissiveDanger.M_Metal_Rust_EmissiveDanger" "None"))
  (bind (_direction _dangertrack) (`Timeline|DangerTimeline` :!via `PlayFromStart`)
    (:`Update`
      (`MaterialInstanceDynamic.SetVectorParameterValue` _returnvalue "EmissiveDanger" (`KismetMathLibrary.MakeColor` _dangertrack)))
    (:`Finished`
      ;[1 1 1] When the gun shoot, it plays shot sound
      (`GameplayStatics.SpawnSoundAtLocation` "/Game/Sounds/SC_ArrowShot.SC_ArrowShot" (`self.K2_GetActorLocation`) (struct) 1.0 1.0 0.4 null null)
      ;[1 1 1] Dart's trajectory
      (bind (_direction_2 _newtrack_0) (`Timeline|ShotTimeline`)
        (:`Update`
          (`SceneComponent.K2_SetRelativeLocation` (`self.DartMesh`) (`KismetMathLibrary.MakeVector` -50.0 (`KismetMathLibrary.Lerp` -250.0 16400.0 _newtrack_0)) false false))))))

(event `self.ReceiveBeginPlay`
  (`KismetSystemLibrary.K2_SetTimerDelegate` (delegate `Fire`) 15.0 true))

(event `self.ReceiveActorBeginOverlap`
  (params (OtherActor :type "Actor Object Reference"))
  ;[1 1 1] Death
  (bind _asfirst_person_character (cast `/Game/FirstPersonBP/Blueprints/FirstPersonCharacter` OtherActor))
  (if (`PrimitiveComponent.IsOverlappingActor` (`self.DartTriggerArea`) _asfirst_person_character)
    (`/Game/FirstPersonBP/Blueprints/FirstPersonCharacter.Death` _asfirst_person_character)
    (else
      (`GameplayStatics.PlaySound2D` "/Game/Sounds/ArrowFlying.ArrowFlying" 1.0 1.0 0.0 null null))))

(fn `UserConstructionScript`)